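; Player character that can make distraction noises and fights enemies through button-prompt quick-time combat.
; IsUnderAttack locks movement, turns the player, shows a random button widget and slows time.
; Correct or wrong presses cost enemy or player a life, looping until one dies, destroying the enemy or quitting the game.
; The B-button check is disconnected, and the elapsed timer never triggers a timeout.
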(event Custom|IsUnderAttack
  (params (WhoIsAttacking :type Actor%20Object%20Reference))
  ;[1 1 1] Stops player from moving in fight
  (Input|SetIgnoreMoveInput (Game|GetPlayerController 0) true)
  ;[1 1 1] Set The Anim State
  (Variables|Default|SetEnemyActor WhoIsAttacking)
  (bind _asenemy_character (Utilities|Casting|CastToEnemyCharacter WhoIsAttacking))
  (bind _ashero_tpp_anim_blueprint (Utilities|Casting|CastToHeroTPP_AnimBlueprint (Components|SkeletalMesh|GetAnimInstance (Variables|/Script/Engine.Character|GetMesh _asenemy_character))))
  (Class|BPAnimINterface|SetAnimationState(Message) _ashero_tpp_anim_blueprint)
  (Utilities|FlowControl|Delay 1.0)
  (Utilities|FlowControl|Sequence
    (:then_0
      ;[1 1 1] Player Faces Enemy In Fight
      (Transformation|SetActorRotation (Class|KismetMathLibrary|MakeRot 0.0 (.Pitch (Class|KismetMathLibrary|BreakRot (Math|Rotator|FindLookatRotation (Transformation|GetActorLocation) (Transformation|GetActorLocation WhoIsAttacking)))) 0.0)))
    (:then_1
      ;[1 1 1] Randomising the Buttons
      (Variables|Default|SetTargetButton (Math|Random|RandomIntegerinRange (Variables|Default|GetMin) (Variables|Default|GetMax))))
    (:then_2
      ;[1 1 1] Link Randomise Button To UIWidget
      (CallFunction|ShowCorrectButtonPress))
    (:then_3
      ;[1 1 1] Start The Timer
      (Variables|Default|SetElapsed%20Time 0.0)
      (Variables|Default|SetIsTiming true))
    (:then_4
      ;[1 1 1] Buttons for fight sequence active
      (Variables|Default|SetIsInCombat true))
    (:then_5
      ;[1 1 1] Slow Down World Time
      (Utilities|Time|SetGlobalTimeDilation 0.5))))

(event EventBeginPlay
  ;[1 1 1] Comment
  (bind _returnvalue (UserInterface|CreateWidget "/Game/UIWIdgets/UIWidget_A.UIWidget_A_C"))
  (Variables|Default|SetWidget%20A _returnvalue)
  (bind _returnvalue_2 (UserInterface|CreateWidget "/Game/UIWIdgets/UIWidget_B.UIWidget_B_C"))
  (Variables|Default|SetWidget%20B _returnvalue_2)
  (bind _returnvalue_3 (UserInterface|CreateWidget "/Game/UIWIdgets/UIWidget_X.UIWidget_X_C"))
  (Variables|Default|SetWidget%20X _returnvalue_3)
  (bind _returnvalue_4 (UserInterface|CreateWidget "/Game/UIWIdgets/UIWidget_Fail.UIWidget_Fail_C"))
  (Variables|Default|SetWidget%20Fail _returnvalue_4)
  (bind _returnvalue_5 (UserInterface|CreateWidget "/Game/UIWIdgets/UIWidget_Collectable.UIWidget_Collectable_C"))
  (Variables|Default|SetWidget%20Collectibles _returnvalue_5)
  (Variables|Default|SetIsInCombat false)
  (Variables|Default|SetIsTiming false))

(event EventTick
  (params (DeltaSeconds :type Float%20%28single-precision%29))
  ;[1 1 1] Setting the Timer
  (if true
    (Variables|Default|SetElapsed%20Time (+ (Variables|Default|GetElapsed%20Time) DeltaSeconds))))

(event Input|ActionEvents|InputActionMakeNoise
  (bind _returnvalue (Game|Player|GetPlayerPawn 0))
  (bind _returnvalue_2 (Transformation|GetActorLocation _returnvalue))
  ;[1 1 1] Making A distraction Noise
  (:Pressed
    (Class|PawnNoiseEmitterComponent|MakeNoise (Variables|Default|GetPawnNoiseEmitter1) (Game|GetPlayerCharacter 0) 1.0 _returnvalue_2)
    (Audio|PlaySoundatLocation "/Game/StarterContent/Audio/Fire01.Fire01" _returnvalue_2)))

(event Input|ActionEvents|InputActionA_Button
  (bind _self self)
  (bind _enemyactor (Variables|Default|GetEnemyActor))
  ;[1 1 1] Check to see if correct button is hit
  (:Pressed
    (if (Variables|Default|GetIsInCombat)
      (if (== (Variables|Default|GetTargetButton) 0)
        ;[1 1 1] Button Pressed Correctly, Reset Combat and Timer back to false
        (CallFunction|SuccessButtonPress)
        (Variables|Default|SetIsInCombat false)
        (Variables|Default|SetIsTiming false)
        ;[1 1 1] Enemy Loses a life
        (Variables|Default|SetEnemy%20Lives (- (Variables|Default|GetEnemy%20Lives) (Variables|Default|GetLose%20Life)))
        ;[1 1 1] Check to see if enemy lives equal 0
        (if (== (Variables|Default|GetEnemy%20Lives) 0)
          ;[1 1 1] If true, play death animation, destroy the enemy and reset the players lives back to 3
          (Input|SetIgnoreMoveInput (Game|GetPlayerController 0) false)
          (bind _asenemy_character (Utilities|Casting|CastToEnemyCharacter _enemyactor))
          (bind _ashero_tpp_anim_blueprint (Utilities|Casting|CastToHeroTPP_AnimBlueprint (Components|SkeletalMesh|GetAnimInstance (Variables|/Script/Engine.Character|GetMesh _asenemy_character))))
          (Class|BPAnimINterface|SetAnimationState(Message) _ashero_tpp_anim_blueprint 5)
          (AI|Components|Blackboard|SetValueasBool (AI|GetBlackboard _asenemy_character) (Variables|Default|GetIsDead) true)
          (Variables|Default|SetEnemyToKill _enemyactor)
          (Utilities|FlowControl|Delay 4.4)
          (Actor|DestroyActor (Variables|Default|GetEnemyToKill))
          (Variables|Default|SetPlayer%20Lives 3)
          (else
            ;[1 1 1] Set The Anim State
            (Utilities|FlowControl|Delay 1.0 :!label _label)
            (Utilities|FlowControl|Sequence
              (:then_0
                ;[1 1 1] Player Faces Enemy In Fight
                (Transformation|SetActorRotation (Class|KismetMathLibrary|MakeRot 0.0 (.Pitch (Class|KismetMathLibrary|BreakRot (Math|Rotator|FindLookatRotation (Transformation|GetActorLocation) (Transformation|GetActorLocation (stale Custom|IsUnderAttack WhoIsAttacking))))) 0.0)))
              (:then_1
                ;[1 1 1] Randomising the Buttons
                (Variables|Default|SetTargetButton (Math|Random|RandomIntegerinRange (Variables|Default|GetMin) (Variables|Default|GetMax))))
              (:then_2
                ;[1 1 1] Link Randomise Button To UIWidget
                (CallFunction|ShowCorrectButtonPress))
              (:then_3
                ;[1 1 1] Start The Timer
                (Variables|Default|SetElapsed%20Time 0.0)
                (Variables|Default|SetIsTiming true))
              (:then_4
                ;[1 1 1] Buttons for fight sequence active
                (Variables|Default|SetIsInCombat true))
              (:then_5
                ;[1 1 1] Slow Down World Time
                (Utilities|Time|SetGlobalTimeDilation 0.5)))))
        (else
          ;[1 1 1] Button pressed incorrectly, combat and timer reset to false
          (CallFunction|FailButtonPress)
          (Utilities|FlowControl|Delay 0.2)
          (Widget|RemovefromParent (Variables|Default|GetWidget%20Fail))
          (Variables|Default|SetIsInCombat false)
          (Variables|Default|SetIsTiming false)
          ;[1 1 1] Player loses a life
          (Variables|Default|SetPlayer%20Lives (- (Variables|Default|GetPlayer%20Lives) (Variables|Default|GetLose%20Life)))
          ;[1 1 1] Check to see if players lives equals 0
          (if (== (Variables|Default|GetPlayer%20Lives) 0)
            ;[1 1 1] Destroy Player and for the moment quit game
            (bind _asmy_character (Utilities|Casting|CastToMyCharacter _self))
            (bind _ashero_tpp_anim_blueprint_2 (Utilities|Casting|CastToHeroTPP_AnimBlueprint (Components|SkeletalMesh|GetAnimInstance (Variables|/Script/Engine.Character|GetMesh _asmy_character))))
            (Class|BPAnimINterface|SetAnimationState(Message) _ashero_tpp_anim_blueprint_2 5)
            (Utilities|FlowControl|Delay 4.4)
            (Actor|DestroyActor _self)
            (Game|QuitGame 0 "Quit")
            (else
              (goto _label))))))))

(event Input|ActionEvents|InputActionB_Button
  ;[1 1 1] Check to see if correct button is hit
)

(event Input|ActionEvents|InputActionX_Button
  (bind _self self)
  (bind _enemyactor (Variables|Default|GetEnemyActor))
  ;[1 1 1] Check to see if correct button is hit
  (:Pressed
    (if (Variables|Default|GetIsInCombat)
      (if (== (Variables|Default|GetTargetButton) 2)
        ;[1 1 1] Button Pressed Correctly, Reset Combat and Timer back to false
        (CallFunction|SuccessButtonPress)
        (Variables|Default|SetIsInCombat false)
        (Variables|Default|SetIsTiming false)
        ;[1 1 1] Enemy Loses a life
        (Variables|Default|SetEnemy%20Lives (- (Variables|Default|GetEnemy%20Lives) (Variables|Default|GetLose%20Life)))
        ;[1 1 1] Check to see if enemy lives equal 0
        (if (== (Variables|Default|GetEnemy%20Lives) 0)
          ;[1 1 1] If true, play death animation, destroy the enemy and reset the players lives back to 3
          (Input|SetIgnoreMoveInput (Game|GetPlayerController 0) false)
          (bind _asenemy_character (Utilities|Casting|CastToEnemyCharacter _enemyactor))
          (bind _ashero_tpp_anim_blueprint (Utilities|Casting|CastToHeroTPP_AnimBlueprint (Components|SkeletalMesh|GetAnimInstance (Variables|/Script/Engine.Character|GetMesh _asenemy_character))))
          (Class|BPAnimINterface|SetAnimationState(Message) _ashero_tpp_anim_blueprint 5)
          (AI|Components|Blackboard|SetValueasBool (AI|GetBlackboard _asenemy_character) (Variables|Default|GetIsDead) true)
          (Variables|Default|SetEnemyToKill _enemyactor)
          (Utilities|FlowControl|Delay 4.4)
          (Actor|DestroyActor (Variables|Default|GetEnemyToKill))
          (Variables|Default|SetPlayer%20Lives 3)
          (else
            ;[1 1 1] Set The Anim State
            (Utilities|FlowControl|Delay 1.0 :!label _label)
            (Utilities|FlowControl|Sequence
              (:then_0
                ;[1 1 1] Player Faces Enemy In Fight
                (Transformation|SetActorRotation (Class|KismetMathLibrary|MakeRot 0.0 (.Pitch (Class|KismetMathLibrary|BreakRot (Math|Rotator|FindLookatRotation (Transformation|GetActorLocation) (Transformation|GetActorLocation (stale Custom|IsUnderAttack WhoIsAttacking))))) 0.0)))
              (:then_1
                ;[1 1 1] Randomising the Buttons
                (Variables|Default|SetTargetButton (Math|Random|RandomIntegerinRange (Variables|Default|GetMin) (Variables|Default|GetMax))))
              (:then_2
                ;[1 1 1] Link Randomise Button To UIWidget
                (CallFunction|ShowCorrectButtonPress))
              (:then_3
                ;[1 1 1] Start The Timer
                (Variables|Default|SetElapsed%20Time 0.0)
                (Variables|Default|SetIsTiming true))
              (:then_4
                ;[1 1 1] Buttons for fight sequence active
                (Variables|Default|SetIsInCombat true))
              (:then_5
                ;[1 1 1] Slow Down World Time
                (Utilities|Time|SetGlobalTimeDilation 0.5)))))
        (else
          ;[1 1 1] Button pressed incorrectly, combat and timer reset to false
          (CallFunction|FailButtonPress)
          (Utilities|FlowControl|Delay 0.2)
          (Widget|RemovefromParent (Variables|Default|GetWidget%20Fail))
          (Variables|Default|SetIsInCombat false)
          (Variables|Default|SetIsTiming false)
          ;[1 1 1] Player loses a life
          (Variables|Default|SetPlayer%20Lives (- (Variables|Default|GetPlayer%20Lives) (Variables|Default|GetLose%20Life)))
          ;[1 1 1] Check to see if players lives equals 0
          (if (== (Variables|Default|GetPlayer%20Lives) 0)
            ;[1 1 1] Destroy Player and for the moment quit game
            (bind _asmy_character (Utilities|Casting|CastToMyCharacter _self))
            (bind _ashero_tpp_anim_blueprint_2 (Utilities|Casting|CastToHeroTPP_AnimBlueprint (Components|SkeletalMesh|GetAnimInstance (Variables|/Script/Engine.Character|GetMesh _asmy_character))))
            (Class|BPAnimINterface|SetAnimationState(Message) _ashero_tpp_anim_blueprint_2 5)
            (Utilities|FlowControl|Delay 4.4)
            (Actor|DestroyActor _self)
            (Game|QuitGame 0 "Quit")
            (else
              (goto _label))))))))

(fn ConstructionScript)

(fn ShowCorrectButtonPress
  (switch int (Variables|Default|GetTargetButton)
    (:0
      (UserInterface|Viewport|AddtoViewport (Variables|Default|GetWidget%20A)))
    (:1
      (UserInterface|Viewport|AddtoViewport (Variables|Default|GetWidget%20B)))
    (:2
      (UserInterface|Viewport|AddtoViewport (Variables|Default|GetWidget%20X)))))

(fn SuccessButtonPress
  (Utilities|FlowControl|Sequence
    (:then_0
      (Utilities|Time|SetGlobalTimeDilation 1.0))
    (:then_1
      (Widget|RemovefromParent (Variables|Default|GetWidget%20A)))))

(fn FailButtonPress
  (Utilities|FlowControl|Sequence
    (:then_0
      (Utilities|Time|SetGlobalTimeDilation 1.0))
    (:then_1
      (Widget|RemovefromParent (Variables|Default|GetWidget%20X)))
    (:then_2
      (UserInterface|Viewport|AddtoViewport (Variables|Default|GetWidget%20Fail)))))

(fn PlayCorrectAnimation)